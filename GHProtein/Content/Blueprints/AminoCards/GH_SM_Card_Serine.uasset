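; Blueprint for a Serine amino acid card, a static mesh object that maps to the Serine residue type.
; Its construction script creates a dynamic material instance on the mesh, and SetFresnel writes a color to that material's Fresnel parameter.
; Type queries report that it is neither a mode toggle nor a temperature lever, and ToEResidue returns the Serine enum value.
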(fn `IsModeToggle`
  (returns (IsToggle :type Boolean))
  (return false))

(fn `IsTempLever`
  (returns (IsLever :type Boolean))
  (return false))

(fn `SetFresnel`
  (params (Color :type "Object.LinearColor Structure"))
  (returns (Completed :type Boolean))
  (`MaterialInstanceDynamic.SetVectorParameterValue` (`self.MaterialInstance`) "Fresnel" Color)
  (return false))

(fn `ToEResidue`
  (returns (Enum :type "ThesisStaticLibrary.EResidueType Enum"))
  (return "kSerine"))

(fn `UserConstructionScript`
  (bind _returnvalue (`PrimitiveComponent.CreateDynamicMaterialInstance` (`self.StaticMesh1`) 0 null))
  (set `self.MaterialInstance` _returnvalue))