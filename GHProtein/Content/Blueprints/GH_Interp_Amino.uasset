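; GH_Interp_Amino is an actor whose mesh, likely an amino acid judging by the name, appears, glides to a target point and disappears.
; SetStopLocation stores the target slightly lowered in Z, and StartInterp moves the initially hidden mesh to a start location, shows it and begins movement.
; Tick eases it toward the target with VInterpTo, then stops and hides it once all axes are within tolerance.
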(event `self.ReceiveTick`
  (params (DeltaSeconds :type "Float (single-precision)"))
  (bind _returnvalue (`KismetMathLibrary.VInterpTo` (`self.CurrentLocation`) (`self.StopV`) DeltaSeconds 1.0))
  (if (`self.IsInterpolating`)
    (`SceneComponent.SetWorldLocation` (`self.StaticMesh1`) _returnvalue false)
    (set `self.CurrentLocation` _returnvalue)
    (if (`KismetMathLibrary.NearlyEqual_FloatFloat` (.x (`self.CurrentLocation`)) (.x (`self.StopV`)) 1.0)
      (if (`KismetMathLibrary.NearlyEqual_FloatFloat` (.y (`self.CurrentLocation`)) (.y (`self.StopV`)) 1.0)
        (if (`KismetMathLibrary.NearlyEqual_FloatFloat` (.z (`self.CurrentLocation`)) (.z (`self.StopV`)) 1.0)
          (set `self.IsInterpolating` false)
          (`SceneComponent.SetVisibility` (`self.StaticMesh1`) false false))))))

(fn `SetStopLocation`
  (params (StopVector :type "Object.Vector Structure"))
  (set `self.StopV` (`KismetMathLibrary.MakeVector` (.x StopVector) (.y StopVector) (- (.z StopVector) 15.0))))

(fn `StartInterp`
  (params (StartLocation :type "Object.Vector Structure"))
  (bind _staticmesh1 (`self.StaticMesh1`))
  (`SceneComponent.SetWorldLocation` _staticmesh1 StartLocation false)
  (set `self.CurrentLocation` StartLocation)
  (`SceneComponent.SetVisibility` _staticmesh1 true false)
  (set `self.IsInterpolating` true))

(fn `UserConstructionScript`
  (`SceneComponent.SetVisibility` (`self.StaticMesh1`) false false)
  (set `self.CurrentLocation` (`SceneComponent.K2_GetComponentLocation` (`self.StaticMesh1`))))