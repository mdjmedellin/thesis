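; GH_SM_Temp_LeverRod is a control-panel lever rod Blueprint that identifies itself as the temp lever through query functions.
; Its construction script creates and stores a dynamic material instance on the static mesh.
; Query functions report it is neither a mode nor secondary toggle and has an unknown residue, while SetFresnel writes a colour to the TempFresnel parameter in the GH_MPC_ControlPanel material parameter collection.
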(fn `IsModeToggle`
  (returns (IsToggle :type Boolean))
  (return false))

(fn `IsSecondaryToggle`
  (returns (IsSecondary :type Boolean))
  (return false))

(fn `IsTempLever`
  (returns (IsLever :type Boolean))
  (set `self.IsLever` true)
  (return (`self.IsLever`)))

(fn `SetFresnel`
  (params (Color :type "Object.LinearColor Structure"))
  (returns (Completed :type Boolean))
  (`KismetMaterialLibrary.SetVectorParameterValue` "/Game/Props/ControlPanel/GH_MPC_ControlPanel.GH_MPC_ControlPanel" "TempFresnel" Color)
  (return false))

(fn `ToEResidue`
  (returns (Enum :type "ThesisStaticLibrary.EResidueType Enum"))
  (return "kUnknownResidue"))

(fn `UserConstructionScript`
  (bind _returnvalue (`PrimitiveComponent.CreateDynamicMaterialInstance` (`self.StaticMesh1`) 0 null))
  (set `self.MaterialInstance` _returnvalue))