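; Camera character Blueprint that edits a custom amino acid chain around a tracked center residue.
; AddResidue inserts after the center and selects the new residue, while the slide functions shift the chain one step, returning the residue type string.
; CenterAminoMaterial highlights the current center and resets the previous one; sliding past either end plays a no-move sound.
; A separate helper translates the protein model to a given spawn location.
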(event `CustomEvent_1`)

(fn `AddResidue`
  (params (Residue :type "EResidueType Enum" :default "kUnknownResidue"))
  (returns (String :type String))
  (set `self.CenterInt` (+ (`self.CenterInt`) 1))
  (`self.AddResidueToCustomChain` Residue true (`self.CenterInt`))
  (set `self.Chainlength` (+ (`self.Chainlength`) 1))
  (`self.CenterAminoMaterial` (- (`self.CenterInt`) 1))
  (bind _returnvalue (`self.GetResidueAtSpecifiedIndex` (`self.CenterInt`)))
  (return (`AminoAcid.GetResidueTypeString` _returnvalue)))

(fn `CenterAminoMaterial`
  (params (OldCenter :type Integer))
  (`|ExecutionSequence`
    (:`then_0`
      (bind _returnvalue (`self.GetResidueAtSpecifiedIndex` (`self.CenterInt`)))
      (bind _asmeshcomponent (cast `MeshComponent` (`KismetArrayLibrary.Array_Get` (`self.K2_GetComponentsByClass` _returnvalue "/Script/Engine.MeshComponent"))))
      (`PrimitiveComponent.SetMaterial` _asmeshcomponent 0 "/Game/Materials/GH_M_CenterAmino.GH_M_CenterAmino"))
    (:`then_1`
      (bind _returnvalue_2 (`self.GetResidueAtSpecifiedIndex` OldCenter))
      (bind _asmeshcomponent_2 (cast `MeshComponent` (`KismetArrayLibrary.Array_Get` (`self.K2_GetComponentsByClass` _returnvalue_2 "/Script/Engine.MeshComponent"))))
      (`PrimitiveComponent.SetMaterial` _asmeshcomponent_2 0 "/Game/Materials/M_Basic_Wall.M_Basic_Wall"))))

(fn `ReturnProteinToSpawn`
  (params (SpawnLocation :type "Object.Vector Structure"))
  (bind _returnvalue (`self.GetProteinModelLocation`))
  (`self.TranslateProteinModel` (`KismetMathLibrary.MakeVector` (- (.x SpawnLocation) (.x _returnvalue)) (- (.y SpawnLocation) (.y _returnvalue)) (- (.z SpawnLocation) (.z _returnvalue)))))

(fn `SlideChainLEft`
  (returns (ToRender :type String))
  (if (< (`self.CenterInt`) (- (`self.Chainlength`) 1))
    (set `self.CenterInt` (+ (`self.CenterInt`) 1))
    (`self.SlideCustomChain` 1)
    (`self.CenterAminoMaterial` (- (`self.CenterInt`) 1))
    (bind _returnvalue (`self.GetResidueAtSpecifiedIndex` (`self.CenterInt`)))
    (return (`AminoAcid.GetResidueTypeString` _returnvalue))
    (else
      (`GameplayStatics.PlaySoundAtLocation` "/Game/Audio/GH_NoMove.GH_NoMove" (-365.0 0.0 -150.0) 0.25))))

(fn `SlideChainRIght`
  (returns (ToRender :type String))
  (if (> (`self.CenterInt`) 0)
    (set `self.CenterInt` (+ (`self.CenterInt`) -1))
    (`self.SlideCustomChain` -1)
    (`self.CenterAminoMaterial` (+ 1 (`self.CenterInt`)))
    (bind _returnvalue (`self.GetResidueAtSpecifiedIndex` (`self.CenterInt`)))
    (return (`AminoAcid.GetResidueTypeString` _returnvalue))
    (else
      (`GameplayStatics.PlaySoundAtLocation` "/Game/Audio/GH_NoMove.GH_NoMove" (-365.0 0.0 -150.0) 0.25))))

(fn `UserConstructionScript`)